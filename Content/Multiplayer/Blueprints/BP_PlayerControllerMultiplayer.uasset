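; Multiplayer player controller that handles spawning, team assignment, respawn and a world-space crosshair for the local player.
; On BeginPlay the local controller requests a pawn and team from BP_GamemodeMultiplayer through server events, then spawns a BP_CrosshairWidget actor.
; PlayerDeath requests another spawn after a short delay, without reassigning the team.
; SetCrosshairlocation moves the crosshair to the supplied trace hit or trace end.
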(event Custom|Set%20Crosshair%20location
  (params (Hit :type Boolean) (Hit%20Location :type Vector) (Trace%20End :type Vector))
  ;[1 0 0] Crosshair: place based on line trace
  ;;[1 1 1] this is done on tick which is not ideal but not too bad for this, called in player controller after calculating the line trace for where the crosshair should be
  (if (Pawn|IsLocalPlayerController)
    ;;[1 1 1] this is a validated get. if this doesn't exist we don't want it to try set the location, this would be when the character is respawning
    (bind _crosshairwidget (Variables|Default|GetCrosshairWidget)
      (:then
        (if Hit
          ;;[1 1 1] crosshair hit something: line it up
          (Transformation|SetActorLocation _crosshairwidget Hit%20Location false false)
          (else
            ;;[1 1 1] crosshair didn't hit anything place it at trace end
            (Transformation|SetActorLocation _crosshairwidget Trace%20End false false))))
      (:else))))

(event Custom|RunOnServer_SpawnPlayer
  ;[0 0.4385 1] Spawn player and Set game mode
  ;;[1 1 1] check to make sure only the server can run this to make sure that players can't hack and add their own players
  (Networking|SwitchHasAuthority
    (:Authority
      ;;[1 1 1] cast gamemode to multiplayer custom gamemode
      (bind _asbp_gamemode_multiplayer (Utilities|Casting|CastToBP_GamemodeMultiplayer (Game|GetGameMode))
        (:then
          (Default|SpawnPlayer _asbp_gamemode_multiplayer self))
        (:CastFailed
          (Development|PrintString "Failed to cast in BP_PlayerController to Gamemode multiplayer when running RunOnServerSpawn" true true "(R=1.000000,G=0.000000,B=0.018970,A=1.000000)"))))))

(event Custom|PlayerDeath
  ;[0 0.4077 1] Respawn players after delay
  (Utilities|FlowControl|Delay 3.0)
  (CallFunction|RunonServerSpawnPlayer))

(event Custom|RunOnServer_SetTeam
  ;[0.4356 0 1] Set team for new players. Runs on gamemode as there is only one instance of it
  (bind _asbp_gamemode_multiplayer (Utilities|Casting|CastToBP_GamemodeMultiplayer (Game|GetGameMode))
    (:then
      (bind _asbp_shooter_character (Utilities|Casting|CastToBP_ShooterCharacter (Pawn|GetControlledPawn))
        (:then
          (Default|SetTeam _asbp_gamemode_multiplayer _asbp_shooter_character))
        (:CastFailed
          (Development|PrintString "cast failed to shooter character before set team"))))
    (:CastFailed
      (Development|PrintString "cast to gamemode failed in spawn player set team"))))

(event EventBeginPlay
  ;[1 1 1] Begin play logic: Spawn player and spawn crosshair actor.
  ;;[1 1 1] if this is copy of controller that is on the server, and not controlled by the server, we do not wan the follwoing code to execute
  (if (Pawn|IsLocalPlayerController)
    ;;[1 1 1] On the server spawn this player that created with this player controller
    (CallFunction|RunonServerSpawnPlayer)
    (CallFunction|RunonServerSetTeam)
    ;;[1 1 1] spawn the crosshair widget and set the reference, get around transform error by spliting the pin.
    (bind _returnvalue (Game|SpawnActorfromClass "/Game/Multiplayer/UI/BP_CrosshairWidget.BP_CrosshairWidget_C" (Math|Transform|MakeTransform "0, 0, 0" "0, 0, 0" "1.000000,1.000000,1.000000") "Undefined" "MultiplyWithRoot" 0 0))
    (Variables|Default|SetCrosshairWidget _returnvalue)))

(fn ConstructionScript)