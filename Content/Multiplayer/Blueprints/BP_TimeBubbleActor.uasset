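; BP_TimeBubbleActor is a temporary time bubble that slows overlapping actors tagged Player or Bullet through CustomTimeDilation, each with its own factor.
; On BeginPlay the visual sphere is sized to the collision radius, and a timeline rate-scaled by BubbleDuration drives actor scale before destroying the bubble.
; Leaving the sphere restores normal speed.
; Destroyed also resets overlapping Pawns, with the Bullet reset nested inside that Pawn loop.
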(event OnComponentBeginOverlap(SphereCollision)
  (params (OverlappedComponent :type Primitive%20Component%20Object%20Reference) (OtherActor :type Actor%20Object%20Reference) (OtherComp :type Primitive%20Component%20Object%20Reference) (OtherBodyIndex :type Integer) (bFromSweep :type Boolean) (SweepResult :type Hit%20Result%20Structure%20%28by%20ref%29))
  ;[1 1 1] if actor overlap is player or bullet set time dilation
  (if (Actor|ActorHasTag OtherActor "Player")
    (Variables|/Script/Engine.Actor|SetCustomTimeDilation OtherActor (Variables|Default|GetPlayerSlowdownFactor))
    (elif (Actor|ActorHasTag OtherActor "Bullet")
      (Variables|/Script/Engine.Actor|SetCustomTimeDilation OtherActor (Variables|Default|GetBulletSlowdownFactor)))))

(event OnComponentEndOverlap(SphereCollision)
  (params (OverlappedComponent :type Primitive%20Component%20Object%20Reference) (OtherActor :type Actor%20Object%20Reference) (OtherComp :type Primitive%20Component%20Object%20Reference) (OtherBodyIndex :type Integer))
  ;[1 1 1] When no longer in bubble set back to normal speed. NOTE: Only works when actors step out of bubble as when actor is destroyed through set lifespan or destory, end overlap will not be called as the collision component is destroyed with the actor
  (Variables|/Script/Engine.Actor|SetCustomTimeDilation OtherActor 1.0))

(event EventBeginPlay
  (bind _spherecollision (Variables|Default|GetSphereCollision))
  (bind _returnvalue (Components|Sphere|GetScaledSphereRadius _spherecollision))
  (bind _returnvalue_2 (/ _returnvalue 5e+01))
  (Development|PrintString "bubel")
  (Transformation|SetWorldScale3D (Variables|Default|GetSphereVisual) (Math|Vector|MakeVector _returnvalue_2 _returnvalue_2 _returnvalue_2))
  ;[1 1 1] use bubble duration divided by 1 so that it scales with the duration of the bubble
  (Components|Timeline|SetPlayRate (Variables|Default|GetBubbleScaleTimeline) (/ 1.0 (Variables|Default|GetBubbleDuration)))
  ;[1 1 1] as long as bubblelifespan
  (bind _shrinkscale (Timeline|BubbleScaleTimeline PlayFromStart)
    (:Update
      (Transformation|SetActorScale3D (Math|Conversions|ToVector(Float) _shrinkscale)))
    (:Finished
      ;[1 1 1] destroy after timeline is finsihed
      (Actor|DestroyActor))))

(event EventDestroyed
  ;[1 1 1] when lifespawn ends or destroyed called set dilation for all charcters and bullets in bubble to normal. (maybe better way to do this idk)
  ;;[1 1 1] reset all players dilation
  (for _array_element (Collision|GetOverlappingActors (Variables|Default|GetSphereCollision) "/Script/Engine.Pawn" :!class /Script/Engine.PrimitiveComponent)
    (Variables|/Script/Engine.Actor|SetCustomTimeDilation _array_element 1.0)
    ;;[1 1 1] reset all bullets dilation
    (for _array_element_2 (Collision|GetOverlappingActors (Variables|Default|GetSphereCollision) "/Game/Multiplayer/Blueprints/bullet.bullet_C" :!class /Script/Engine.PrimitiveComponent)
      (Variables|/Script/Engine.Actor|SetCustomTimeDilation _array_element_2 1.0))))

(fn ConstructionScript)