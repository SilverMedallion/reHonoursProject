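; BP_PlayerStateMultiplayer is a multiplayer player state Blueprint that holds a player's team name, team colour and personal score.
; SetTeam stores the team identity, while IncreasePlayerScore overwrites PersonalScore with the increment instead of adding to it.
; The getters for game activity, time remaining, team and scores are stubs that return fixed default values rather than the stored variables.
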(event EventIncreasePlayerScore
  (params (Increment :type Integer))
  (Variables|Default|SetPersonalScore Increment))

(event EventSetTeam
  (params (TeamName :type TeamNames%20Enum :default "NewEnumerator0") (TeamColour :type Linear%20Color%20Structure))
  ;[1 1 1] set team name and colour
  (Variables|Default|SetTeamName TeamName)
  (Variables|Default|SetTeamColour TeamColour))

(fn ConstructionScript)

(fn GetGameIsActive
  (return false))

(fn GetGameTimeRemaining
  (return 0))

(fn GetPlayerScore
  (return 0))

(fn GetTeam
  (return "NewEnumerator0" ""))

(fn GetTeamScore
  (return 0))