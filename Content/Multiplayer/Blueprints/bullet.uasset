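; Multiplayer bullet actor that detects hits with a short forward line trace every tick, run only on the server.
; A blocking hit branches on physical surface: Body and Head spawn blood and apply damage, higher for Head, with the bullet's owner as damage causer.
; Concrete and other surfaces spawn an asphalt impact effect, and every blocking hit destroys the bullet.
; Traces are left drawn as persistent debug lines.
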(event EventBeginPlay)

(event Collision|EventActorBeginOverlap
  (params (OtherActor :type Actor%20Object%20Reference)))

(event EventTick
  (params (DeltaSeconds :type Float%20%28single-precision%29))
  (bind _returnvalue (Transformation|GetActorLocation))
  ;[1 1 1] every tick fire a line trace from the front of the bullet
  ;;[1 1 1] only run this tick on the server so the clients don't have to pass it between them
  (Networking|SwitchHasAuthority
    (:Authority
      (bind _outhit (Collision|LineTraceByChannel _returnvalue (+ _returnvalue (* (Transformation|GetActorForwardVector) 1.8e+02)) "TraceTypeQuery1" false 0 "Persistent"))
      (if (.bblockinghit _outhit)
        (switch Utilities|FlowControl|Switch|SwitchonEPhysicalSurface (Variables|/Script/PhysicsCore.PhysicalMaterial|GetSurfaceType (.physmat _outhit))
          (:SurfaceType_Default
            (Effects|SpawnEmitteratLocation "/Game/Realistic_Starter_VFX_Pack_Vol2/Particles/Hit/P_Asphalt.P_Asphalt" (.location _outhit) (Math|Rotator|Delta(Rotator) (Math|Conversions|RotationFromXVector (.normal _outhit)) "90.000000,0.000000,0.000000") :!label _label))
          (:SurfaceType1
            ;[1 1 1] body hit
            (Effects|SpawnEmitteratLocation "/Game/Realistic_Starter_VFX_Pack_Vol2/Particles/Blood/P_Blood_Splat_Cone.P_Blood_Splat_Cone" (.location _outhit) (Math|Rotator|Delta(Rotator) (Math|Conversions|RotationFromXVector (.normal _outhit)) "90.000000,0.000000,0.000000"))
            (Game|Damage|ApplyDamage (.hitactor _outhit) 2e+01 0 (Components|GetOwner) "/Script/Engine.DamageType"))
          (:SurfaceType2
            (goto _label))
          (:SurfaceType4
            ;[1 1 1] head hit
            (Effects|SpawnEmitteratLocation "/Game/Realistic_Starter_VFX_Pack_Vol2/Particles/Blood/P_Blood_Splat_Cone.P_Blood_Splat_Cone" (.location _outhit) (Math|Rotator|Delta(Rotator) (Math|Conversions|RotationFromXVector (.normal _outhit)) "90.000000,0.000000,0.000000"))
            (Game|Damage|ApplyDamage (.hitactor _outhit) 5e+01 0 (Components|GetOwner) "/Script/Engine.DamageType")))
        (Actor|DestroyActor)))))

(fn ConstructionScript)