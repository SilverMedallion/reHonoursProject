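; Multiplayer bullet actor that spawns impact effects and applies damage when its box collider hits something.
; The hit's physical surface selects the response: blood plus damage for Body or Head, asphalt particles otherwise, then the bullet destroys itself.
; Damage is higher for Head, though that call has no damaged actor wired, and names the bullet's owner as causer.
; Overlap stores the other actor and runs a short forward trace whose result is unused.
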(event OnComponentHit(BoxCollider)
  (params (HitComponent :type Primitive%20Component%20Object%20Reference) (OtherActor :type Actor%20Object%20Reference) (OtherComp :type Primitive%20Component%20Object%20Reference) (NormalImpulse :type Vector :default "0, 0, 0") (Hit :type Hit%20Result%20Structure%20%28by%20ref%29))
  (bind _returnvalue (Math|Conversions|RotationFromXVector (.normal Hit)))
  (bind _returnvalue_2 (Math|Rotator|Delta(Rotator) _returnvalue "90.000000,0.000000,0.000000"))
  (switch Utilities|FlowControl|Switch|SwitchonEPhysicalSurface (Variables|/Script/PhysicsCore.PhysicalMaterial|GetSurfaceType (.physmat Hit))
    (:SurfaceType_Default
      (Effects|SpawnEmitteratLocation "/Game/Realistic_Starter_VFX_Pack_Vol2/Particles/Hit/P_Asphalt.P_Asphalt" (.location Hit) _returnvalue_2 :!label _label))
    (:SurfaceType1
      ;[1 1 1] body hit
      (Effects|SpawnEmitteratLocation "/Game/Realistic_Starter_VFX_Pack_Vol2/Particles/Blood/P_Blood_Splat_Cone.P_Blood_Splat_Cone" (.location Hit) _returnvalue_2)
      (Game|Damage|ApplyDamage (.hitactor Hit) 2e+01 0 (Components|GetOwner) "/Script/Engine.DamageType"))
    (:SurfaceType2
      (goto _label))
    (:SurfaceType4
      ;[1 1 1] head hit
      (Effects|SpawnEmitteratLocation "/Game/Realistic_Starter_VFX_Pack_Vol2/Particles/Blood/P_Blood_Splat_Cone.P_Blood_Splat_Cone" (.location Hit) _returnvalue_2)
      (Game|Damage|ApplyDamage 0 5e+01 0 (Components|GetOwner) "/Script/Engine.DamageType")))
  (Actor|DestroyActor))

(event OnComponentBeginOverlap(BoxCollider)
  (params (OverlappedComponent :type Primitive%20Component%20Object%20Reference) (OtherActor :type Actor%20Object%20Reference) (OtherComp :type Primitive%20Component%20Object%20Reference) (OtherBodyIndex :type Integer) (bFromSweep :type Boolean) (SweepResult :type Hit%20Result%20Structure%20%28by%20ref%29))
  (bind _returnvalue (Transformation|GetActorLocation))
  (bind _output_get (Variables|Default|SetHitActor OtherActor))
  (Collision|LineTraceByChannel _returnvalue (+ _returnvalue (* (Math|Vector|GetForwardVector (Variables|Default|GetDefaultSceneRoot self)) 1.0)) "TraceTypeQuery1" false 0 "None"))

(fn ConstructionScript)