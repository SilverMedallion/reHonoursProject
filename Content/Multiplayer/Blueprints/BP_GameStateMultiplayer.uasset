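; Multiplayer game state that tracks the round countdown, Blue and Red team scores, and rounds won.
; BeginPlay starts a looping one-second timer on authority, which decrements GameTimer, then pauses itself and calls EndRound on BP_GamemodeMultiplayer.
; Authority-gated events increment team scores and round wins, with each round win also calling EndRound.
; The score and round-win OnRep functions and the RunOnServer_StartRoundTimer event are empty stubs.
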(event Custom|RunOnServer_AddScoreToTeam
  (params (Team :type TeamNames%20Enum :default "NewEnumerator0"))
  ;[1 1 1] Score. team scores that increase with each kill
  (Networking|SwitchHasAuthority
    (:Authority
      (switch Utilities|FlowControl|Switch|SwitchonTeamNames Team
        (:NewEnumerator0
          (Variables|Default|SetTeamBlueScore (+ (Variables|Default|GetTeamBlueScore) 1)))
        (:NewEnumerator1
          (Variables|Default|SetTeamRedScore (+ (Variables|Default|GetTeamRedScore) 1)))))))

(event Custom|RunOnServer_AddRoundWinToTeam
  (params (RoundWinningTeam :type TeamNames%20Enum :default "NewEnumerator0"))
  ;[1 1 1] Rounds. Team round win count that should increase at the end of each round
  (Networking|SwitchHasAuthority
    (:Authority
      (switch Utilities|FlowControl|Switch|SwitchonTeamNames RoundWinningTeam
        (:NewEnumerator0
          (Variables|Default|SetTeamBlueRoundsWon (+ (Variables|Default|GetTeamBlueRoundsWon) 1))
          (bind _asbp_gamemode_multiplayer (Utilities|Casting|CastToBP_GamemodeMultiplayer (Game|GetGameMode))
            (:then
              (Default|EndRound _asbp_gamemode_multiplayer))
            (:CastFailed
              (Development|PrintString "Failed to cast to gamemode in game state round end" true true "(R=1.000000,G=0.000000,B=0.000000,A=1.000000)" 1e+01))))
        (:NewEnumerator1
          (Variables|Default|SetTeamRedRoundsWon (+ (Variables|Default|GetTeamRedRoundsWon) 1))
          (bind _asbp_gamemode_multiplayer_2 (Utilities|Casting|CastToBP_GamemodeMultiplayer (Game|GetGameMode))
            (:then
              (Default|EndRound _asbp_gamemode_multiplayer_2))
            (:CastFailed
              (Development|PrintString "Failed to cast to gamemode in game state round end" true true "(R=1.000000,G=0.000000,B=0.000000,A=1.000000)" 1e+01))))))))

(event Custom|RunOnServer_StartRoundTimer
  ;[1 1 1] StartRoundTimer currently not called, need to call this when we want a round to start.
)

(event Custom|UpdateTimer
  ;[1 1 1] While game timer is > 0 subtract 1. This is called by the timer started in RunOnServer_StartRoundTimer every second
  (if (> (Variables|Default|GetGameTimer) 0)
    (Variables|Default|SetGameTimer (- (Variables|Default|GetGameTimer) 1))
    (else
      ;[1 1 1] Call game timer done so stop checking score in gamemodepuase timer when game ends so end game doesn't loop getting called
      (Variables|Default|SetGameTimerDone true)
      (Utilities|Time|PauseTimerbyHandle (Variables|Default|GetTimerRef))
      ;[1 1 1] don't use rep notify here as it is calling end round from the gamemode which only exists on client. If want other functionality to run on the clients would want to reread the replicating variables in blueprint doc
      (bind _asbp_gamemode_multiplayer (Utilities|Casting|CastToBP_GamemodeMultiplayer (Game|GetGameMode))
        (:then
          (Default|EndRound _asbp_gamemode_multiplayer))
        (:CastFailed
          (Development|PrintString "Failed to cast to gamemode in game state update timer" true true "(R=1.000000,G=0.000000,B=0.000000,A=1.000000)" 1e+01))))))

(event EventBeginPlay
  ;[1 1 1] StartRoundTimer currently not called, need to call this when we want a round to start.
  ;;[1 1 1] just trying begin play for now(works it seems)
  ;[1 1 1] Comment
  (Utilities|Casting|CastToBP_GamemodeMultiplayer (Game|GetGameMode)
    (:then
      (Networking|SwitchHasAuthority
        (:Authority
          (bind _returnvalue (Utilities|Time|SetTimerbyFunctionName 0 "UpdateTimer" 1.0 true))
          ;[1 1 1] store timer to stop it on game end
          (Variables|Default|SetTimerRef _returnvalue))))
    (:CastFailed
      ;;[1 0 0.2462] THIS CAST IS FAILING CURRENTLY!!!
      (Development|PrintString "Failed to cast to gamemode in game state begin play" true true "(R=1.000000,G=0.000000,B=0.000000,A=1.000000)" 1e+01))))

(fn ConstructionScript)

(fn OnRepTeamRedScore)

(fn OnRepTeamBlueScore)

(fn OnRepTeamBlueRoundsWon)

(fn OnRepTeamRedRoundsWon)