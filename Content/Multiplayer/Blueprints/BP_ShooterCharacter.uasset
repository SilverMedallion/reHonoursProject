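; Player character for a multiplayer shooter with aim-down-sights, sprint, a slow-motion dive and a cooldown-gated time bubble.
; Input calls server RPCs for speed, pitch, bullet spawning and bubbles, while a local muzzle trace places the crosshair.
; Server-side damage updates RepNotify health for the UI, multicasts hit reactions and ragdoll death, and awards team score through the game state.
; Hitscan firing and the motion-warped TimeDive remain but are disconnected.
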(event Custom|RunOnServer_SetPitch
  (params (Pitch :type Float%20%28double-precision%29))
  ;[1 0.9994 0] Pitch Control: set pitch when look input action triggerd, run the set pitch on server fro the pitch change, multicast back to all the clients the players changed ptich
  ;;[1 1 1] set to reliable and run on server to make it a "remote procedure call/rpc" so it's being called to run on the server. Then call multicast to actually set the pitch
  (CallFunction|MulticastSetPitch Pitch))

(event Custom|Multicast_SetPitch
  (params (Pitch :type Float%20%28double-precision%29))
  ;[1 0.9994 0] Pitch Control: set pitch when look input action triggerd, run the set pitch on server fro the pitch change, multicast back to all the clients the players changed ptich
  ;;[1 1 1] set pitch replication to replicated
  (Variables|Default|SetPitch Pitch))

(event Custom|Multicast_SpawnBubble
  ;[0 0.9546 1] Time Bubble stuuf
  ;;[1 1 1] spawn bubble for clients
  (CallFunction|TimeBubble (Variables|Default|GetMuzzleTransform)))

(event Custom|RunOnServer_Dive
  (Networking|SwitchHasAuthority
    (:Authority
      (CallFunction|TimeDive))))

(event Custom|RunOnClient_CreateUI
  ;[0 1 0.05132] UI: health bar set up on client
  (bind _returnvalue (UserInterface|CreateWidget "/Game/Multiplayer/UI/WBP_GameplayUI.WBP_GameplayUI_C" (Variables|Default|GetBP%20Player%20Controller%20Multiplayer%20Ref)))
  (bind _output_get (Variables|Default|SetGameplayUIRef _returnvalue))
  (UserInterface|Viewport|AddtoViewport _output_get 0)
  (Default|BindHealth _output_get)
  ;[1 1 1] ensure health displays correctly from the start
  (Default|CallHealthChanged (Variables|Default|GetHealth)))

(event Custom|RunOnServer_AimingSpeedChange
  (params (Action%20Value :type Boolean))
  (bind _charactermovement (Variables|Character|GetCharacterMovement))
  ;[1 0 0] max walk speed is part of charcter movement which server has authority on so must be ran on server
  (if Action%20Value
    ;;[1 1 1] slow down move speed when aiming and speed up when released
    (Variables|/Script/Engine.CharacterMovementComponent|SetMaxWalkSpeed _charactermovement (Variables|Default|GetAimSpeed))
    (else
      (Variables|/Script/Engine.CharacterMovementComponent|SetMaxWalkSpeed _charactermovement (Variables|Default|GetRunSpeed)))))

(event Custom|RunOnServer_Sprint
  (params (Action%20Value :type Boolean))
  (bind _charactermovement (Variables|Character|GetCharacterMovement))
  ;[1 0.9799 0.9479] Sprint logic: must run on server for max walk speed as server authoritive over character movement component
  (if Action%20Value
    ;;[1 1 1] Set speed to sprint speed when held, run speed when releaesd
    (Variables|/Script/Engine.CharacterMovementComponent|SetMaxWalkSpeed _charactermovement (Variables|Default|GetSprintSpeed))
    (else
      (Variables|/Script/Engine.CharacterMovementComponent|SetMaxWalkSpeed _charactermovement (Variables|Default|GetRunSpeed)))))

(event Custom|CustomEvent
  (params (MuzzleTransform :type Transform))
  ;[1 0.2098 0] OLD: Shooting from Muzzle logic, call for applied damage and spawn muzzle flash effects here
  ;;[1 1 1] want fire to be done on server so players cannot hack and change their own fire
)

(event Custom|Multicast_SpawnFXs
  (params (Hit :type Boolean) (HitLocation :type Vector) (HitNormal :type Vector) (PhysicalMaterial :type Physical%20Material%20Object%20Reference))
  (bind _returnvalue (Math|Conversions|RotationFromXVector HitNormal))
  (bind _returnvalue_2 (Math|Rotator|Delta(Rotator) _returnvalue "90.000000,0.000000,0.000000"))
  ;[1 0 0.7923] effects  for shooting such as sounds and impact marks
  ;;[1 1 1] Dont want any of this stuff to run on dedicated server as only clients need it
  (if (not (Networking|IsDedicatedServer))
    ;;[1 1 1] play gunshot sound
    (Audio|PlaySoundatLocation "/Game/Sounds/M4Gunshot.M4Gunshot" (Variables|Default|GetFireLocation) "0, 0, 0" 1.0 1.0 0.0 0 0 0 0)
    ;;[1 1 1] stuff after this will only run if we hit something
    (if Hit
      ;;[1 1 1] Switch for different physics materials of object hit. TODO: add different effect for metal
      (switch Utilities|FlowControl|Switch|SwitchonEPhysicalSurface (Variables|/Script/PhysicsCore.PhysicalMaterial|GetSurfaceType PhysicalMaterial)
        (:SurfaceType_Default
          ;;[1 1 1] basic impact effect
          (Effects|SpawnEmitteratLocation "/Game/Realistic_Starter_VFX_Pack_Vol2/Particles/Hit/P_Asphalt.P_Asphalt" HitLocation _returnvalue_2 "0.400000,0.400000,0.400000" :!label _label)
          ;;[1 1 1] sounds for hits. TODO: make different sounds.
          (Audio|PlaySoundatLocation "/Game/Sounds/BulletRicochet.BulletRicochet" HitLocation "0, 0, 0" 1.0 1.0 0.0 0 0 0 0))
        (:SurfaceType1
          ;;[1 1 1] Blood effect
          (Effects|SpawnEmitteratLocation "/Game/Realistic_Starter_VFX_Pack_Vol2/Particles/Blood/P_Blood_Splat_Cone.P_Blood_Splat_Cone" HitLocation _returnvalue_2 "0.400000,0.400000,0.400000")
          (Audio|PlaySoundatLocation "/Game/Sounds/BulletRicochet.BulletRicochet" HitLocation "0, 0, 0" 1.0 1.0 0.0 0 0 0 0))
        (:SurfaceType2
          (goto _label))
        (:SurfaceType3
          (goto _label))))))

(event Custom|RunOnServer_AnyDamage
  (params (Damage :type Float%20%28double-precision%29) (DamageCauser :type Actor%20Object%20Reference))
  ;[1 0.2098 0] Damage and death logic here
  ;;[1 1 1] Run when player takes damage
  ;;;[1 1 1] check for authority to avoid clients cheating
  (Networking|SwitchHasAuthority
    (:Authority
      ;;[1 1 1] check player is alive before running on server
      (if (Variables|Default|GetAlive)
        ;;[1 1 1] subtract health when hit. Health is replicated with notify. When health is changed OnRep_Health is called
        (Variables|Default|SetHealth (- (Variables|Default|GetHealth) Damage))
        (CallFunction|MulticastAnyDamage)
        ;;[1 1 1] kill players when health 0
        (if (<= (Variables|Default|GetHealth) 0.0)
          (Variables|Default|SetAlive false)
          ;;[1 1 1] call death event
          (CallFunction|MulticastDeath)
          (bind _asbp_game_state_multiplayer (Utilities|Casting|CastToBP_GameStateMultiplayer (Game|GetGameState)))
          (bind _ascharacter (Utilities|Casting|CastToCharacter DamageCauser)
            (:then
              (bind _asbp_player_state_multiplayer (Utilities|Casting|CastToBP_PlayerStateMultiplayer (Variables|/Script/Engine.Pawn|GetPlayerState _ascharacter))
                (:then
                  ;[1 1 1] General score increaes for ui and such
                  (Default|RunonServerAddScoretoTeam _asbp_game_state_multiplayer (Variables|/Game/Multiplayer/Blueprints/BP_PlayerStateMultiplayer.BP_PlayerStateMultiplayer_C|GetAssignedTeam _asbp_player_state_multiplayer))
                  ;[1 1 1] round increase for respawning and game ending
                  (Default|RunonServerAddRoundWintoTeam _asbp_game_state_multiplayer (Variables|/Game/Multiplayer/Blueprints/BP_PlayerStateMultiplayer.BP_PlayerStateMultiplayer_C|GetAssignedTeam _asbp_player_state_multiplayer)))
                (:CastFailed
                  (Development|PrintString "Cast in event any damage to player state is failing" true true "(R=1.000000,G=0.000000,B=0.017682,A=1.000000)" 5.0))))
            (:CastFailed
              (Development|PrintString "Cast in event any damage to player character failed"))))))))

(event Custom|Multicast_AnyDamage
  ;[1 0.2098 0] Damage and death logic here
  ;;[1 1 1] Run when player takes damage
  ;;;[1 1 1] play taking damage montage
  (Animation|Montage|PlayMontage (Variables|Character|GetMesh) "/Game/AnimStarterPack/UE5/UE5_Hit_React_1_Montage.UE5_Hit_React_1_Montage"))

(event Custom|Multicast_Death
  (bind _mesh (Variables|Character|GetMesh))
  ;[1 0.2098 0] Damage and death logic here
  ;;[1 1 1] on death: ragdol and set on collisoin and disable player input
  (Physics|SetSimulatePhysics _mesh true)
  (Class|SkeletalMeshComponent|SetPhysicsBlendWeight _mesh 1.0)
  (Collision|SetCollisionEnabled _mesh "QueryAndPhysics")
  (Collision|SetCollisionEnabled (Variables|Default|GetCapsuleComponent) "NoCollision")
  (Input|DisableInput (Game|GetPlayerController 0)))

(event Custom|RunOnServer_Fire
  (params (MuzzleTransform :type Transform))
  ;[1 0.2098 0] Shooting from Muzzle logic, spawn bullet, call for applied damage and spawn muzzle flash effects here
  ;;[1 1 1] want fire to be done on server so players cannot hack and change their own fire
  ;;[1 1 1] check what is running fire has authority to make sure it's server to stop cheating( get rid of this for now to do new aurthoirty for line trace stuff
  (Networking|SwitchHasAuthority
    (:Authority
      ;;[1 1 1] have muzzle transform replicated over the network
      (bind _output_get (Variables|Default|SetMuzzleTransform MuzzleTransform))
      ;;[1 1 1] spawn in bullet actor which will fly out and hit
      (CallFunction|SpawnBullet _output_get))))

(event Custom|RunOnServer_FireBubble
  (params (MuzzleTransform :type Transform))
  ;[0 0.9546 1] Time Bubble stuuf
  ;;[1 1 1] Gonna have this run on server since not sure exactly how tis gonna turn out if it's a spawned actor or not. If it is a spawned actor system it shouldn't need this as a actor spawn in automatically replicated however if it's a line trace system it's gonna need this
  (Networking|SwitchHasAuthority
    (:Authority
      (Variables|Default|SetMuzzleTransform MuzzleTransform)
      (CallFunction|MulticastSpawnBubble))))

(event Custom|SpawnBullet
  (params (MuzzleTransform :type Transform))
  ;[1 0.2098 0] Shooting from Muzzle logic, spawn bullet, call for applied damage and spawn muzzle flash effects here
  ;;[1 1 1] multicast to spawn the bullets for all clients, object spawning is automattically replicated so function is not a multicast
  (Game|SpawnActorfromClass "/Game/Multiplayer/Blueprints/bullet.bullet_C" MuzzleTransform "Undefined" "MultiplyWithRoot" self self))

(event Input|EnhancedActionEvents|EnhancedInputActionIA_Look
  (params (ActionValue :type Vector%202D%20Structure) (ElapsedSeconds :type Float%20%28double-precision%29) (TriggeredSeconds :type Float%20%28double-precision%29) (InputAction :type Input%20Action%20Object%20Reference :default "/Game/ThirdPerson/Input/Actions/IA_Look.IA_Look"))
  ;[1 0.9994 0] Pitch Control: set pitch when look input action triggerd, run the set pitch on server fro the pitch change, multicast back to all the clients the players changed ptich
  ;;[1 1 1] When look triggered set pitch for the player on server so other players can see
  (CallFunction|RunonServerSetPitch (.pitch (Pawn|GetControlRotation :!class /Script/Engine.Pawn))))

(event Input|EnhancedActionEvents|EnhancedInputActionIA_AimDownSights
  (params (ActionValue :type Boolean) (ElapsedSeconds :type Float%20%28double-precision%29) (TriggeredSeconds :type Float%20%28double-precision%29) (InputAction :type Input%20Action%20Object%20Reference :default "/Game/ThirdPerson/Input/Actions/IA_AimDownSights.IA_AimDownSights"))
  (bind _cameraboom (Variables|Default|GetCameraBoom))
  (bind _cameraboom_2 (Variables|Default|GetCameraBoom))
  ;[1 0 0] Aim down sights logic
  ;;[1 1 1] character movement can only be edited on server
  (CallFunction|RunonServerAimingSpeedChange ActionValue)
  (if ActionValue
    ;;[1 1 1] move socket offset using a timeline, it's current offset will be it's start point
    (Variables|/Script/Engine.SpringArmComponent|SetSocketOffset _cameraboom (Variables|/Script/Engine.SpringArmComponent|GetSocketOffset _cameraboom))
    ;;[1 1 1] when clicking right mouse if already executing a timeline it wil l stop that one and start the other
    (Utilities|FlowControl|Sequence
      (:then_0
        (bind _newtrack_0 (Timeline|Timeline_0 Stop)
          (:Update
            ;;[1 1 1] set to 75 on y and z as on camera boom 75 is the socket offset that is set by default ot give the over the sholder cam
            (Variables|/Script/Engine.SpringArmComponent|SetSocketOffset _cameraboom_2 (Math|Vector|MakeVector (Math|Float|Lerp (.x (Variables|/Script/Engine.SpringArmComponent|GetSocketOffset (Variables|Default|GetCameraBoom))) 0.0 _newtrack_0) 75.0 75.0)))))
      (:then_1
        ;;;[1 1 1] time line float track goes from 0 to 0.25 at finishin
        (bind _newtrack_0_2 (Timeline|Timeline PlayFromStart)
          (:Update
            (Variables|/Script/Engine.SpringArmComponent|SetSocketOffset _cameraboom_2 (Math|Vector|MakeVector (Math|Float|Lerp (.x (Variables|/Script/Engine.SpringArmComponent|GetSocketOffset (Variables|Default|GetCameraBoom))) (Variables|Default|GetADSMagnification) _newtrack_0_2) 75.0 75.0))))))
    (else
      (Variables|/Script/Engine.SpringArmComponent|SetSocketOffset _cameraboom (Variables|/Script/Engine.SpringArmComponent|GetSocketOffset _cameraboom))
      (Utilities|FlowControl|Sequence
        (:then_0
          (Timeline|Timeline Stop))
        (:then_1
          (Timeline|Timeline_0 PlayFromStart))))))

(event Input|EnhancedActionEvents|EnhancedInputActionIA_Fire
  (params (ActionValue :type Boolean) (ElapsedSeconds :type Float%20%28double-precision%29) (TriggeredSeconds :type Float%20%28double-precision%29) (InputAction :type Input%20Action%20Object%20Reference :default "/Game/ThirdPerson/Input/Actions/IA_Fire.IA_Fire"))
  ;[1 0.2098 0] when fire is pressed run the fire on server and pass in the transfrom of the bun muzzle at the time
  (if ActionValue
    (CallFunction|RunonServerFire (Transformation|GetSocketTransform (Variables|Default|GetWeapon) "b_gun_muzzleflashSocket" "RTS_World"))))

(event Input|EnhancedActionEvents|EnhancedInputActionIA_Sprint
  (params (ActionValue :type Boolean) (ElapsedSeconds :type Float%20%28double-precision%29) (TriggeredSeconds :type Float%20%28double-precision%29) (InputAction :type Input%20Action%20Object%20Reference :default "/Game/ThirdPerson/Input/Actions/IA_Sprint.IA_Sprint"))
  ;[1 0.9799 0.9479] Sprint logic: must run on server for max walk speed as server authoritive over character movement component
  (CallFunction|RunonServerSprint ActionValue))

(event Input|EnhancedActionEvents|EnhancedInputActionIA_Dive
  (params (ActionValue :type Boolean) (ElapsedSeconds :type Float%20%28double-precision%29) (TriggeredSeconds :type Float%20%28double-precision%29) (InputAction :type Input%20Action%20Object%20Reference :default "/Game/ThirdPerson/Input/Actions/IA_Dive.IA_Dive"))
  (bind _charactermovement (Variables|Character|GetCharacterMovement))
  ;[0.09824 0.2292 0.013] Dive input.
  (Variables|Default|SetbUseControllerRotationYaw false)
  (Variables|Default|SetIsDiving true)
  ;;[1 1 1] Calculate Dive Vector to lauch character
  (bind _output_get (Variables|Default|SetDiveVector (Math|Vector|MakeVector (.x (* (Variables|Default|GetDiveLaunchSpeed) (Transformation|GetActorForwardVector))) 0.0 (Variables|Default|GetDiveHeight))))
  (Character|LaunchCharacter _output_get false false)
  ;;[1 1 1] Adjust Air control and gravity during dive as appropriate
  (Variables|/Script/Engine.CharacterMovementComponent|SetAirControl _charactermovement 0.3)
  (Variables|/Script/Engine.CharacterMovementComponent|SetGravityScale _charactermovement 1.2)
  ;;[1 1 1] set global dilation
  (Utilities|Time|SetGlobalTimeDilation 0.5))

(event Input|EnhancedActionEvents|EnhancedInputActionIA_TimeBubble
  (params (ActionValue :type Boolean) (ElapsedSeconds :type Float%20%28double-precision%29) (TriggeredSeconds :type Float%20%28double-precision%29) (InputAction :type Input%20Action%20Object%20Reference :default "/Game/ThirdPerson/Input/Actions/IA_TimeBubble.IA_TimeBubble"))
  ;[0 0.9546 1] Time Bubble stuuf
  ;;[1 1 1] check cooldown is finsihed before firing
  (if (Variables|Default|GetBubbleCooldownElapsed)
    (CallFunction|RunonServerFireBubble (Transformation|GetSocketTransform (Variables|Default|GetWeapon) "b_gun_muzzleflashSocket" "RTS_World"))
    ;;[1 1 1] allow player to use bubble after cooldown has ended
    (Variables|Default|SetBubbleCooldownElapsed false)
    (Utilities|FlowControl|Delay (Variables|Default|GetBubbleCooldownDuration))
    (Variables|Default|SetBubbleCooldownElapsed true)))

(event Input|EnhancedActionEvents|EnhancedInputActionIA_Menu
  (params (ActionValue :type Boolean) (ElapsedSeconds :type Float%20%28double-precision%29) (TriggeredSeconds :type Float%20%28double-precision%29) (InputAction :type Input%20Action%20Object%20Reference :default "/Game/ThirdPerson/Input/Actions/IA_Menu.IA_Menu"))
  (bind _returnvalue (Game|GetPlayerController 0))
  ;[1 1 1] If puase menu has been used don't need to create it just set input mode to ui
  (Variables|Default|GetPauseMenuRef
    (:then
      _)
    (:else
      (bind _returnvalue_2 (UserInterface|CreateWidget "/Game/Multiplayer/UI/WBP_PauseMenu.WBP_PauseMenu_C"))
      (bind _output_get (Variables|Default|SetPauseMenuRef _returnvalue_2))))
  (Variables|/Script/Engine.PlayerController|SetbShowMouseCursor _returnvalue true)
  (Input|SetInputModeUIOnly _returnvalue _output_get "DoNotLock" false)
  (UserInterface|Viewport|AddtoViewport _output_get 0))

(event EventBeginPlay
  ;[1 1 1] overwrite default player controller in networked time shooter character c++ class ith new multiplayer player controller
  ;;[1 1 1] need to delay till next tick as on begin play there will not be a controller created yet so the mapping context will not work correctly
  (Utilities|FlowControl|DelayUntilNextTick)
  (if (Pawn|IsLocallyControlled)
    (bind _asbp_player_controller_multiplayer (Utilities|Casting|CastToBP_PlayerControllerMultiplayer (Pawn|GetController))
      (:then
        ;;[1 1 1] store multiplayer player controller as variable
        (Variables|Default|SetBP%20Player%20Controller%20Multiplayer%20Ref _asbp_player_controller_multiplayer)
        (Utilities|IsValid (PlayerController|LocalPlayerSubsystems|GetEnhancedInputLocalPlayerSubsystem _asbp_player_controller_multiplayer)
          (:Is%20Valid
            ;;[1 0.9994 0] add mapping contect for the player controller, needed for input actions to work
            (Input|AddMappingContext (PlayerController|LocalPlayerSubsystems|GetEnhancedInputLocalPlayerSubsystem _asbp_player_controller_multiplayer) "/Game/ThirdPerson/Input/IMC_Default.IMC_Default" 0 "(bIgnoreAllPressedKeysUntilRelease=True,bForceImmediately=False,bNotifyUserSettings=False)")
            ;[1 1 1] Check valid as if not will cause crash when respawning.
            (bind _gameplayuiref (Variables|Default|GetGameplayUIRef)
              (:then
                ;[1 1 1] Must bind health on create ui as well as here so when character respawns health bar is still updated
                (Default|BindHealth _gameplayuiref))
              (:else)))))
      (:CastFailed
        (Development|PrintString "ERROR: BP_ShooterCharacter after begin play. Cast failed for controller to PlayerControllerMultiplayer. ")))))

(event EventPossessed
  (params (NewController :type Controller%20Object%20Reference))
  ;[0 1 0.05132] UI: health bar set up on client
  (CallFunction|RunonClientCreateUI))

(event EventOnLanded
  (params (Hit :type Hit%20Result%20Structure%20%28by%20ref%29))
  (bind _charactermovement (Variables|Character|GetCharacterMovement))
  ;[0.09824 0.2292 0.013] Dive input.
  ;;[1 1 1] set diving to false when landing to transition back to normal state. NOTE: is diving in the abp is set to the is diving from here.
  (Variables|Default|SetIsDiving false)
  (Utilities|Time|SetGlobalTimeDilation 1.0)
  (Variables|/Script/Engine.CharacterMovementComponent|SetAirControl _charactermovement 0.0)
  (Variables|/Script/Engine.CharacterMovementComponent|SetGravityScale _charactermovement 1.0))

(event Game|Damage|EventAnyDamage
  (params (Damage :type Float%20%28single-precision%29) (DamageType :type Damage%20Type%20Object%20Reference) (InstigatedBy :type Controller%20Object%20Reference) (DamageCauser :type Actor%20Object%20Reference))
  ;[1 0.2098 0] Damage and death logic here
  ;;[1 1 1] Run when player takes damage
  ;;;[1 1 1] fire anytime damage is applied to character
  (CallFunction|RunonServerAnyDamage Damage DamageCauser))

(event EventTick
  (params (DeltaSeconds :type Float%20%28single-precision%29))
  (bind _weapon (Variables|Default|GetWeapon))
  (bind _returnvalue (Transformation|GetSocketTransform _weapon "b_gun_muzzleflashSocket" "RTS_World"))
  ;[1 0 0] CROSSHAIR: trace the location for crosshair placement every tick
  (if (and (Pawn|IsLocallyControlled) (not (Networking|IsDedicatedServer)))
    ;;[1 1 1] get weapon muzzle socket at end of gun and do a drace from the end of it to then pass into set crosshair for placement calculations
    (bind (_outhit _returnvalue_2) (Collision|LineTraceByChannel (.location _returnvalue) (+ (.location _returnvalue) (* (Math|Vector|GetForwardVector (.rotation _returnvalue)) (Variables|Default|GetFireRange))) "TraceTypeQuery3" false 0 "None" true "(R=1.000000,G=0.000000,B=0.000000,A=1.000000)" "(R=0.000000,G=1.000000,B=0.000000,A=1.000000)" 2.0))
    (bind _bp_player_controller_multiplayer_ref (Variables|Default|GetBP%20Player%20Controller%20Multiplayer%20Ref)
      (:then
        (Default|SetCrosshairLocation _bp_player_controller_multiplayer_ref _returnvalue_2 (.Location (Collision|BreakHitResult _outhit)) (.TraceEnd (Collision|BreakHitResult _outhit))))
      (:else
        (Development|PrintString "BP_ShooterCharacter. Player controler reference is not valid in crosshair setup")))))

(fn ConstructionScript
  (Transformation|AttachComponentToComponent (Variables|Default|GetWeapon) (Variables|Character|GetMesh) "gun_socket" "SnapToTarget" "SnapToTarget" "SnapToTarget" true))

(fn SetAppliedDamage
  (params (DamagedActor :type Actor%20Object%20Reference) (PhysicalMaterial :type Physical%20Material%20Object%20Reference) (HIt :type Boolean))
  ;[1 1 1] will cause errors if we don't check if something has been hit
  (if HIt
    (switch Utilities|FlowControl|Switch|SwitchonEPhysicalSurface (Variables|/Script/PhysicsCore.PhysicalMaterial|GetSurfaceType PhysicalMaterial)
      (:SurfaceType1
        ;[1 1 1] apply damage
        (Game|Damage|ApplyDamage DamagedActor (Variables|Default|GetWeaponBodyDamage) 0 self "/Script/Engine.DamageType"))
      (:SurfaceType4
        (Game|Damage|ApplyDamage DamagedActor (Variables|Default|GetWeaponHeadDamage) 0 self "/Script/Engine.DamageType")))))

(fn TimeBubble
  (params (MuzzleTransform :type Transform))
  (bind _outhit (Collision|LineTraceByChannel (.location MuzzleTransform) (+ (.location MuzzleTransform) (* (Math|Vector|GetForwardVector (Variables|Default|GetFollowCamera)) (Variables|Default|GetBubbleRange))) "TraceTypeQuery1" false 0 "Persistent" true "(R=1.000000,G=0.000000,B=0.000000,A=1.000000)" "(R=0.000000,G=1.000000,B=0.000000,A=1.000000)" 1e+01))
  (Game|SpawnActorfromClass "/Game/Multiplayer/Blueprints/BP_TimeBubbleActor.BP_TimeBubbleActor_C" (Math|Transform|MakeTransform (.ImpactPoint (Collision|BreakHitResult _outhit)) "0, 0, 0" "1.000000,1.000000,1.000000") "Undefined" "MultiplyWithRoot" self 0))

(fn ResetTimeDilation
  (Variables|Default|SetCustomTimeDilation 1.0)
  (return))

(fn TimeDive
  (bind _returnvalue (Transformation|GetActorLocation))
  (bind _returnvalue_2 (Transformation|GetActorForwardVector))
  (bind _f_forwardoffset (LocalVariables|GetF%20ForwardOffset))
  (bind _f_zoffset (LocalVariables|GetF%20ZOffset))
  (bind _returnvalue_3 (* _returnvalue_2 _f_forwardoffset))
  (bind _returnvalue_4 (+ _returnvalue _returnvalue_3))
  (bind (_x _y _z) (Math|Vector|BreakVector _returnvalue_4))
  (bind _returnvalue_5 (+ _z _f_zoffset))
  (bind _returnvalue_6 (Math|Vector|MakeVector _x _y _returnvalue_5))
  (if (not (Variables|Default|GetDivePlaying))
    (Variables|Default|SetDivePlaying true)
    (Pawn|Components|CharacterMovement|SetMovementMode (Variables|Character|GetCharacterMovement) "MOVE_Flying" 0)
    ;[1 1 1] set so mouse doesn't rotate player while diving
    (Variables|Default|SetbUseControllerRotationYaw true)
    (Variables|Default|SetbUseControllerRotationRoll false)
    (Variables|Default|SetbUseControllerRotationPitch true)
    ;[1 1 1] set mid point for dive calculations
    (LocalVariables|SetMid%20Point _returnvalue_6)
    (Class|MotionWarpingComponent|AddorUpdateWarpTargetfromTransform (Variables|Default|GetMotionWarping) "MotionWarping" (Math|Transform|MakeTransform _returnvalue_6 (Transformation|GetActorRotation) "1.000000,1.000000,1.000000"))
    (bind _outhit (Collision|LineTraceByChannel (+ (* (Math|Vector|GetForwardVector (Variables|Default|GetDiveForwardArrow)) (LocalVariables|GetF%20ForwardOffset)) (LocalVariables|GetMid%20Point)) (+ (+ (* (Math|Vector|GetForwardVector (Variables|Default|GetDiveForwardArrow)) (LocalVariables|GetF%20ForwardOffset)) (LocalVariables|GetMid%20Point)) (Math|Vector|MakeVector 0.0 0.0 (LocalVariables|GetDownRange))) "TraceTypeQuery1" false 0 "ForDuration"))
    (Class|MotionWarpingComponent|AddorUpdateWarpTargetfromTransform (Variables|Default|GetMotionWarping) "MotionWarpingReturn" (Math|Transform|MakeTransform (.ImpactPoint (Collision|BreakHitResult _outhit)) (Transformation|GetActorRotation) "1.000000,1.000000,1.000000"))
    (bind _returnvalue_7 (Animation|PlayAnimMontage "/Game/Multiplayer/Animations/Dive/AM_DiveMontage.AM_DiveMontage" 1.0 "None"))
    (Utilities|Time|SetTimerbyEvent (EventDispatchers|CreateEvent :!event TimeDiveFinished) _returnvalue_7)))

(fn TimeDiveFinished
  (Utilities|Time|SetGlobalTimeDilation 1.0)
  (Pawn|Components|CharacterMovement|SetMovementMode (Variables|Character|GetCharacterMovement) "MOVE_Walking" 0)
  (Variables|Default|SetbUseControllerRotationYaw true)
  (Variables|Default|SetbUseControllerRotationRoll true)
  (Variables|Default|SetbUseControllerRotationPitch true)
  (Variables|Default|SetDivePlaying false)
  (return))

(fn OnRepHealth
  (bind _newhealth (CallFunction|GetHealthPercentage))
  ;[1 1 1] call health changed event in gameplay UI blueprint
  (Default|CallHealthChanged _newhealth)
  (Development|PrintString (Utilities|String|Append "Health changed to" (Utilities|String|ToString(Float) _newhealth)))
  (return))

(fn GetHealthPercentage
  ;[1 1 1] set to pure so it doensn't require an execution pin
  (return (/ (Variables|Default|GetHealth) (Variables|Default|GetMaxHealth))))